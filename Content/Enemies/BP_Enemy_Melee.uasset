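; Sword-wielding melee enemy, built on a parent enemy, with slash, predictive jump and chasing spin attacks, the default being the slash.
; Montage notifies trigger sphere-trace damage, the arced leap, the spin and its AOE slash, and sword spawn or removal on equip and unequip.
; BPC_Attacks applies trace damage, while BPC_DamageSystem handles incoming damage, interruptibility and chance-based blocking with a timed hold.
; Death turns the mesh into a ragdoll.
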(event `self.ReceiveBeginPlay`
  (`parent.ReceiveBeginPlay`))

(event `self.DefaultAttack`
  (params (AttackTarget :type "Actor Object Reference"))
  ;[1 1 1] Attack Animation
  (`self.ShortRangeAttack` AttackTarget))

(event `ShortRangeAttack`
  (params (AttackTarget :type "Actor Object Reference"))
  ;[1 1 1] Attack Animation
  (`parent.DefaultAttack` AttackTarget)
  (bind _notifyname (`|PlayMontage` (`self.Mesh`) "/Game/Animations/Melee/Montage_Sword_Slash.Montage_Sword_Slash")
    (:`then`
      (set `/Game/DamageSystem/BPC_DamageSystem.IsInterruptible` false (`self.BPC_DamageSystem`)))
    (:`OnCompleted`
      (`self.AttackEnd` AttackTarget :!label _label)
      (set `/Game/DamageSystem/BPC_DamageSystem.IsInterruptible` true (`self.BPC_DamageSystem`)))
    (:`OnInterrupted`
      (goto _label))
    (:`OnNotifyBegin`
      (switch `name` _notifyname
        (:`Slash`
          (`self.SphereTraceDamage`))))))

(event `LongRangeAttack`
  (params (AttackTarget :type "Actor Object Reference"))
  ;[1 1 1] Attack Animation
  (`parent.DefaultAttack` AttackTarget)
  (bind _notifyname (`|PlayMontage` (`self.Mesh`) "/Game/Animations/Melee/Montage_Sword_Jump_Attack.Montage_Sword_Jump_Attack")
    (:`then`
      (set `/Game/DamageSystem/BPC_DamageSystem.IsInterruptible` false (`self.BPC_DamageSystem`)))
    (:`OnCompleted`
      (`self.AttackEnd` AttackTarget :!label _label_2)
      (set `/Game/DamageSystem/BPC_DamageSystem.IsInterruptible` true (`self.BPC_DamageSystem`)))
    (:`OnInterrupted`
      (goto _label_2))
    (:`OnNotifyBegin`
      (switch `name` _notifyname
        (:`Slash`
          (`self.SphereTraceDamage`))
        (:`Jump`
          (`self.JumpToAttackTarget` AttackTarget))))))

(event `SphereTraceDamage`
  (bind _returnvalue (`self.K2_GetActorLocation`))
  ;[1 1 1] Attack Helpers
  (bind (_outhits _returnvalue_2) (`KismetSystemLibrary.SphereTraceMultiForObjects` :`Start` _returnvalue :`End` (+ _returnvalue (* (`self.GetActorForwardVector`) 200.0)) :`Radius` 20.0 :`ObjectTypes` (`|MakeArray` "ObjectTypeQuery3" :!type "EObjectTypeQuery Enum") :`DrawDebugType` "ForDuration"))
  (if _returnvalue_2
    (`/Game/Attacks/BPC_Attacks.DamageAllNonTeamMembers` (`self.BPC_Attacks`) _outhits (make `/Game/DamageSystem/S_DamageInfo` 1.0 "NewEnumerator1" "NewEnumerator0" false true true))))

(event `SpinningAttack`
  (params (AttackTarget :type "Actor Object Reference"))
  ;[1 1 1] Attack Animation
  (`parent.DefaultAttack` AttackTarget)
  (bind _notifyname (`|PlayMontage` (`self.Mesh`) "/Game/Animations/Melee/Montage_Sword_SpinningAttack.Montage_Sword_SpinningAttack")
    (:`then`
      (set `/Game/DamageSystem/BPC_DamageSystem.IsInterruptible` true (`self.BPC_DamageSystem`)))
    (:`OnCompleted`
      (`self.AttackEnd` AttackTarget :!label _label_3)
      (set `/Game/DamageSystem/BPC_DamageSystem.IsInterruptible` true (`self.BPC_DamageSystem`))
      (`self.StopSpinning`))
    (:`OnInterrupted`
      (goto _label_3))
    (:`OnNotifyBegin`
      (switch `name` _notifyname
        (:`Slash`
          (`self.SphereTraceDamage`))
        (:`Spin`
          (`self.SpinMesh`)
          (`self.ChaseAttackTarget` AttackTarget))
        (:`AOESlash`
          (`self.AOESlash` AttackTarget))))))

(event `JumpToAttackTarget`
  (params (AttackTarget :type "Actor Object Reference"))
  ;[1 1 1] Attack Helpers
  (bind _location (`self.CalculateFutureActorLocation` AttackTarget))
  (bind _outlaunchvelocity (`GameplayStatics.SuggestProjectileVelocity_CustomArc` (`self.K2_GetActorLocation`) (`KismetMathLibrary.MakeVector` (.x _location) (.y _location) (+ (.z _location) 100.0))))
  (`self.LaunchCharacter` _outlaunchvelocity true true)
  (add `self.LandedDelegate` (delegate `OnLand`)))

(event `OnLand` :!signature `self.LandedDelegate`
  (params (Hit :type "HitResult Structure (by ref)"))
  ;[1 1 1] Attack Helpers
  (remove `self.LandedDelegate` (delegate `OnLand`))
  (`MovementComponent.StopMovementImmediately` (`self.CharacterMovement`)))

(event `SpinMesh`
  (bind (_meshrotationbeforespin_roll _meshrotationbeforespin_pitch _meshrotationbeforespin_yaw) (`KismetMathLibrary.BreakRotator` (`self.MeshRotationBeforeSpin`)))
  ;[1 1 1] Attack Helpers
  (set `self.MeshRotationBeforeSpin` (`SceneComponent.RelativeRotation` (`self.Mesh`)))
  (bind (_direction _zrotationalpha) (`Timeline|SpinMeshTimeline` :!via `PlayFromStart`)
    (:`Update`
      (`SceneComponent.K2_SetRelativeRotation` (`self.Mesh`) (`KismetMathLibrary.MakeRotator` _meshrotationbeforespin_roll _meshrotationbeforespin_pitch) false false))))

(event `self.EquipWeapon`
  ;[1 1 1] Spawns Weapon
  (bind _notifyname (`|PlayMontage` (`self.Mesh`) "/Game/Characters/Mannequins/Animations/Manny/UnSheathingSword_UE_Montage.UnSheathingSword_UE_Montage")
    (:`OnCompleted`
      (`self.OnWeaponEquipped`))
    (:`OnNotifyBegin`
      (switch `name` _notifyname
        (:`GrabSword`
          (bind _returnvalue (`|SpawnActorFromClass` "/Game/Weapons/MyOwnWeaponBase/BP_OwnWeapon_Sword.BP_OwnWeapon_Sword_C" (`self.GetTransform`) "Undefined" "MultiplyWithRoot" null null))
          (bind _output_get (set `self.WeaponActor` _returnvalue))
          (`self.K2_AttachToComponent` _output_get (`self.Mesh`) "hand_r_sword_socket" "SnapToTarget" "SnapToTarget" "SnapToTarget" true)
          (set `self.isWieldingWeapon` true))))))

(event `StopSpinning`
  ;[1 1 1] Attack Helpers
  (`TimelineComponent.Stop` (`self.SpinMeshTimeline`))
  (`SceneComponent.K2_SetRelativeRotation` (`self.Mesh`) (`self.MeshRotationBeforeSpin`) false false))

(event `ChaseAttackTarget`
  (params (AttackTarget :type "Actor Object Reference"))
  ;[1 1 1] Attack Helpers
  (`|AIMoveTo` self (0.0 0.0 0.0) AttackTarget 200.0
    (:`OnSuccess`
      (`KismetSystemLibrary.Delay` 0.1)
      (if (`self.Attacking`)
        (`self.ChaseAttackTarget` AttackTarget)))))

(event `self.UnequipWeapon`
  ;[1 1 1] Despawns Weapon
  (bind _notifyname (`|PlayMontage` (`self.Mesh`) "/Game/Characters/Mannequins/Animations/Manny/SheathingSword_UE_Montage.SheathingSword_UE_Montage")
    (:`OnCompleted`
      (`self.OnWeaponUnequipped`))
    (:`OnNotifyBegin`
      (switch `name` _notifyname
        (:`DropSword`
          (`self.K2_DestroyActor` (`self.WeaponActor`))
          (set `self.isWieldingWeapon` false))))))

(event `AOESlash`
  (params (AttackTarget :type "Actor Object Reference"))
  ;[1 1 1] Attack Helpers
  (bind _returnvalue (`|SpawnActorFromClass` "/Game/AOE/BP_AOE_Base.BP_AOE_Base_C" (`KismetMathLibrary.MakeTransform` (`self.K2_GetActorLocation`)) "Undefined" "MultiplyWithRoot" null true false false self))
  (set `/Game/AOE/BP_AOE_Base.Radius` 300.0 _returnvalue)
  (add `/Game/AOE/BP_AOE_Base.OnAOEOverlapActor` _returnvalue (delegate `AOEDamageActor`))
  (`/Game/AOE/BP_AOE_Base.Trigger` _returnvalue))

(event `AOEDamageActor`
  (params (Actor :type "Actor Object Reference"))
  ;[1 1 1] Attack Helpers
  (if (== Actor (stale `AOESlash` AttackTarget))
    (message `/Game/DamageSystem/BPI_Damageable.TakeDamage` Actor (make `/Game/DamageSystem/S_DamageInfo` 10.0 "NewEnumerator1" "NewEnumerator1") self)))

(event `StartBlock`
  (params (canBeParried :type Boolean))
  ;[1 1 1] Blocking
  (`KismetSystemLibrary.K2_ClearAndInvalidateTimerHandle` (`self.HoldBlockTimer`))
  (`MovementComponent.StopMovementImmediately` (`self.CharacterMovement`))
  (set `/Game/DamageSystem/BPC_DamageSystem.IsBlocking` true (`self.BPC_DamageSystem`))
  (set `self.BlockingState` "NewEnumerator1")
  (`MovementComponent.StopMovementImmediately` (`self.CharacterMovement`))
  (bind _returnvalue (`KismetSystemLibrary.K2_SetTimerDelegate` (`|CreateDelegate` :!event `EndBlock`) 2.0))
  (set `self.HoldBlockTimer` _returnvalue))

(event `self.BPC_DamageSystem.OnBlocked`
  (params (canBeParried :type Boolean) (DamageDealer :type "Actor Object Reference"))
  ;[1 1 1] Blocking
  (set `self.BlockingState` "NewEnumerator2")
  (`KismetSystemLibrary.K2_ClearAndInvalidateTimerHandle` (`self.HoldBlockTimer`))
  (`|PlayMontage` (`self.Mesh`) "/Game/Animations/Melee/Montage_Sword_Block_React.Montage_Sword_Block_React"
    (:`OnCompleted`
      _)
    (:`OnInterrupted`
      _))
  (`self.EndBlock`))

(event `EndBlock`
  ;[1 1 1] Blocking
  (set `/Game/DamageSystem/BPC_DamageSystem.IsBlocking` false (`self.BPC_DamageSystem`))
  (set `self.BlockingState` "NewEnumerator0")
  (`self.OnBlockEnded`))

(event `Death`
  (bind _mesh (`self.Mesh`))
  ;[1 1 1] Death
  (`PrimitiveComponent.SetSimulatePhysics` _mesh true)
  (`PrimitiveComponent.SetCollisionEnabled` _mesh "QueryAndPhysics"))

(fn `CalculateFutureActorLocation`
  (params (Actor :type "Actor Object Reference") (Time :type "Float (double-precision)" :default 1.0))
  (returns (Location :type "Vector Structure"))
  (return (+ (`self.K2_GetActorLocation` Actor) (* (* (`self.GetVelocity` Actor) (1.0 1.0 0.0)) Time))))

(fn `GetIdealRange`
  (returns (AttackRadius :type "Float (double-precision)") (`Defend/StrafeRadius` :type "Float (double-precision)"))
  (return 200.0 400.0))

(fn `TakeDamage`
  (params (DamageInfo :type "/Game/DamageSystem/S_DamageInfo Structure") (DamageDealer :type "Actor Object Reference"))
  (returns (WasDamaged :type Boolean))
  (if (`.CanBeBlocked_13_C0FCA21A4410E487C4E2DD9526E15D1A` (break `/Game/DamageSystem/S_DamageInfo` DamageInfo))
    (`self.TryToBlock`))
  (bind _wasdamaged (`/Game/DamageSystem/BPC_DamageSystem.TakeDamage` (`self.BPC_DamageSystem`) DamageInfo DamageDealer))
  (return _wasdamaged))

(fn `TryToBlock`
  (if (<= (`KismetMathLibrary.RandomFloat`) (`self.BlockChance`))
    (`self.StartBlock` false)))

(fn `UserConstructionScript`
  (`parent.UserConstructionScript`)
  (set `self.MeshRotationBeforeSpin` (`SceneComponent.RelativeRotation` (`self.Mesh`))))